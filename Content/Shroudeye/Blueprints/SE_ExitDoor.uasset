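; SE_ExitDoor is an exit door actor whose Door component switches between a blocking and an open state.
; On BeginPlay, the Block flag decides whether the door starts visible with collision or hidden without it.
; The EventEscapeDoor event reapplies both settings from the ExitDoor flag, hiding the door and disabling collision when it is true, restoring them otherwise.
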(event `EventEscapeDoor`
  (bind _exitdoor_ (`self.ExitDoor?`))
  (`SceneComponent.SetVisibility` (`self.Door`) (not _exitdoor_) false)
  (`PrimitiveComponent.SetCollisionEnabled` (`self.Door`) (select `bool` _exitdoor_ :`false` "QueryAndPhysics" :`true` "NoCollision" :!type "ECollisionEnabled Enum")))

(event `self.ReceiveBeginPlay`
  (`SceneComponent.SetVisibility` (`self.Door`) (`self.Block?`) false)
  (`PrimitiveComponent.SetCollisionEnabled` (`self.Door`) (select `bool` (`self.Block?`) :`false` "NoCollision" :`true` "QueryAndPhysics" :!type "ECollisionEnabled Enum")))

(fn `UserConstructionScript`)